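; Audio hallucination manager actor that plays random phantom sounds around the player character at irregular intervals.
; A timer with a random delay between configured bounds is scheduled on BeginPlay and again after each play attempt.
; Each attempt rolls against a play chance and, on success, spawns a random entry from the sound array at a random direction and distance from the player.
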(event Custom|Schedule%20Next%20Hallucination
  (Utilities|Time|SetTimerbyEvent (EventDispatchers|CreateEvent :!event Custom|Try%20Play%20Hallucination) (Math|Random|RandomFloatinRange (Variables|Default|GetMinDelay) (Variables|Default|GetMaxDelay))))

(event Custom|Try%20Play%20Hallucination
  (bind _hallucinationsounds (Variables|Default|GetHallucinationSounds))
  (if (<= (Math|Random|RandomFloatinRange 0.0 1.0) (Variables|Default|GetChanceToPlay))
    (bind _output_get (Variables|Default|SetChosenIndex (Math|Random|RandomIntegerinRange 0 (Utilities|Array|LastIndex _hallucinationsounds))))
    (Audio|SpawnSoundatLocation (Utilities|Array|Get(acopy) _hallucinationsounds _output_get) (+ (Transformation|GetActorLocation (Game|GetPlayerCharacter 0)) (* (Math|Random|RandomUnitVector) (Math|Random|RandomFloatinRange (Variables|Default|GetMinRadius) (Variables|Default|GetMaxRadius)))) "0, 0, 0" 1.0 1.0 0.0 0 0)
    (CallFunction|ScheduleNextHallucination)
    (else
      (CallFunction|ScheduleNextHallucination))))

(event EventBeginPlay
  (CallFunction|ScheduleNextHallucination))

(fn ConstructionScript)