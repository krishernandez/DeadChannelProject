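; BP_InteractObject is a collectible pickup that counts toward a win condition.
; When the first-person character overlaps its Box, it increments that character's PickUps counter and destroys itself.
; Once the count reaches ten, it shows the WBP_WinMenu widget, pauses the game and switches to a mouse-driven, UI-only input mode.
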(event OnComponentBeginOverlap(Box)
  (params (OverlappedComponent :type Primitive%20Component%20Object%20Reference) (OtherActor :type Actor%20Object%20Reference) (OtherComp :type Primitive%20Component%20Object%20Reference) (OtherBodyIndex :type Integer) (bFromSweep :type Boolean) (SweepResult :type Hit%20Result%20Structure%20%28by%20ref%29))
  (bind _asbp_first_person_character (Utilities|Casting|CastToBP_FirstPersonCharacter OtherActor))
  (Variables|/Game/FirstPerson/Blueprints/BP_FirstPersonCharacter.BP_FirstPersonCharacter_C|SetPickUps _asbp_first_person_character (+ (Variables|/Game/FirstPerson/Blueprints/BP_FirstPersonCharacter.BP_FirstPersonCharacter_C|GetPickUps _asbp_first_person_character) 1))
  (Actor|DestroyActor)
  (if (>= (Variables|/Game/FirstPerson/Blueprints/BP_FirstPersonCharacter.BP_FirstPersonCharacter_C|GetPickUps _asbp_first_person_character) 10)
    (bind _returnvalue (UserInterface|CreateWidget "/Game/UI/WBP_WinMenu.WBP_WinMenu_C"))
    (UserInterface|Viewport|AddtoViewport _returnvalue 0)
    (Game|SetGamePaused true)
    (Variables|/Script/Engine.PlayerController|SetbShowMouseCursor (Game|GetPlayerController 0) true)
    (Input|SetInputModeUIOnly 0 0 "DoNotLock" false)))

(fn ConstructionScript)